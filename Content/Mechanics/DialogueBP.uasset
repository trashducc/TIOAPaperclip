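; DialogueBP is an actor that shows location-based dialogue widgets when the player overlaps its three collision volumes: house exit, in front of work and office building.
; The house exit sets a shared 2ndCollision flag on first visit, switching it and the work volume to alternate lines; the office line is fixed.
; Each line clears after a delay via RemoveAllWidgets, which also runs on every overlap before the player check.
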(event OnComponentBeginOverlap(DialogueCollision)
  (params (OverlappedComponent :type Primitive%20Component%20Object%20Reference) (OtherActor :type Actor%20Object%20Reference) (OtherComp :type Primitive%20Component%20Object%20Reference) (OtherBodyIndex :type Integer) (bFromSweep :type Boolean) (SweepResult :type Hit%20Result%20Structure%20%28by%20ref%29))
  ;[1 1 1] Dialogue1 (Exit of House)
  (Viewport|RemoveAllWidgets)
  (if (== OtherActor (Game|GetPlayerCharacter 0))
    (if (Variables|Default|Get2ndCollision?)
      (UserInterface|Viewport|AddtoViewport (Variables|Default|GetDialogue5) 0)
      (Utilities|FlowControl|Delay 5.0)
      (Viewport|RemoveAllWidgets)
      (else
        (UserInterface|Viewport|AddtoViewport (Variables|Default|GetDialogue1) 0)
        (Variables|Default|Set2ndCollision? true)
        (Utilities|FlowControl|Delay 5.0)
        (Viewport|RemoveAllWidgets)))))

(event OnComponentBeginOverlap(DialogueCollision2)
  (params (OverlappedComponent :type Primitive%20Component%20Object%20Reference) (OtherActor :type Actor%20Object%20Reference) (OtherComp :type Primitive%20Component%20Object%20Reference) (OtherBodyIndex :type Integer) (bFromSweep :type Boolean) (SweepResult :type Hit%20Result%20Structure%20%28by%20ref%29))
  ;[1 1 1] Dialogue 2 (In front of work)
  (Viewport|RemoveAllWidgets)
  (if (== OtherActor (Game|GetPlayerCharacter 0))
    (if (Variables|Default|Get2ndCollision?)
      (UserInterface|Viewport|AddtoViewport (Variables|Default|GetDialogue6) 0)
      (Utilities|FlowControl|Delay 3.0)
      (Viewport|RemoveAllWidgets)
      (else
        (UserInterface|Viewport|AddtoViewport (Variables|Default|GetDialogue2) 0)
        (Utilities|FlowControl|Delay 3.0)
        (Viewport|RemoveAllWidgets)))))

(event OnComponentBeginOverlap(DialogueCollision3)
  (params (OverlappedComponent :type Primitive%20Component%20Object%20Reference) (OtherActor :type Actor%20Object%20Reference) (OtherComp :type Primitive%20Component%20Object%20Reference) (OtherBodyIndex :type Integer) (bFromSweep :type Boolean) (SweepResult :type Hit%20Result%20Structure%20%28by%20ref%29))
  ;[1 1 1] Dialogue 3 (Office building)
  (Viewport|RemoveAllWidgets)
  (if (== OtherActor (Game|GetPlayerCharacter 0))
    (UserInterface|Viewport|AddtoViewport (Variables|Default|GetDialogue3) 0)
    (Utilities|FlowControl|Delay 5.0)
    (Viewport|RemoveAllWidgets)))

(event EventBeginPlay)

(event Collision|EventActorBeginOverlap
  (params (OtherActor :type Actor%20Object%20Reference)))

(event EventTick
  (params (DeltaSeconds :type Float%20%28single-precision%29)))

(fn ConstructionScript)